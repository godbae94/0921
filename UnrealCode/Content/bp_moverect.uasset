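; Actor Blueprint that moves its static mesh around a square loop in the vertical XZ plane.
; Each Tick, a switch on the Movetype enum steps the X or Z location by a fixed amount and applies it as the mesh's relative location.
; Reaching a limit advances the state in the cycle Right, Up, Left, Down.
; Movement is per frame without delta time, so speed follows frame rate.
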(event `self.ReceiveBeginPlay`)

(event `self.ReceiveTick`
  (params (DeltaSeconds :type "Float (single-precision)"))
  (switch `/Game/en_movetype` (`self.movetype`)
    (:`NewEnumerator0`
      ;[1 1 1] 오른쪽으로 움직이기
      (bind _output_get (set `self.x_location` (+ (`self.x_location`) 2.0)))
      (`SceneComponent.K2_SetRelativeLocation` (`self.StaticMesh`) (`KismetMathLibrary.MakeVector` _output_get) false false)
      ;[1 1 1] 만약 x위치가 200과같거나크면 트루를 실행 //
      ; movetype에서 up을 실행한다.
      (if (>= (`self.x_location`) 200.0)
        (set `self.movetype` "NewEnumerator1")))
    (:`NewEnumerator1`
      ;[1 1 1] 위쪽으로 움직이기
      (bind _output_get_2 (set `self.z_location` (+ (`self.z_location`) 2.0)))
      (`SceneComponent.K2_SetRelativeLocation` (`self.StaticMesh`) (`KismetMathLibrary.MakeVector` (`self.x_location`) 0.0 _output_get_2) false false)
      (if (>= (`self.z_location`) 200.0)
        (set `self.movetype` "NewEnumerator2")))
    (:`NewEnumerator2`
      ;[1 1 1] 왼쪽으로 움직이기
      (bind _output_get_3 (set `self.x_location` (+ (`self.x_location`) -2.0)))
      (`SceneComponent.K2_SetRelativeLocation` (`self.StaticMesh`) (`KismetMathLibrary.MakeVector` _output_get_3 0.0 (`self.z_location`)) false false)
      (if (<= (`self.x_location`) 0.0)
        (set `self.movetype` "NewEnumerator3")))
    (:`NewEnumerator3`
      ;[1 1 1] 아래쪽으로 움직이기
      (bind _output_get_4 (set `self.z_location` (+ (`self.z_location`) -2.0)))
      (`SceneComponent.K2_SetRelativeLocation` (`self.StaticMesh`) (`KismetMathLibrary.MakeVector` (`self.x_location`) 0.0 _output_get_4) false false)
      (if (<= (`self.z_location`) 0.0)
        (set `self.movetype` "NewEnumerator0")))))

(fn `UserConstructionScript`)