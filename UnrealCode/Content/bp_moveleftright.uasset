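; Moving object Blueprint that slides its static mesh back and forth along relative X while a linked Switch is active.
; BeginPlay binds to the Switch's overlap dispatcher, or prints a red error naming the actor if none is assigned; EventOverlap sets Isplay from the overlap state.
; While Isplay is set, Tick steps X by a fixed per-frame amount, independent of delta time, flipping direction at two hard-coded limits.
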(event `self.ReceiveBeginPlay`
  (bind _switch (`self.Switch`))
  ;[1 1 1] 이벤트에 바인딩(이벤트를 팔로우한다)
  (`/Engine/EditorBlueprintResources/StandardMacros.IsValid` _switch
    (:`Is Valid`
      (add `/Game/bp_switch.EventDispatcher_Overlap` _switch (`|CreateDelegate` :!event `EventOverlap`)))
    (:`Is Not Valid`
      (`KismetSystemLibrary.PrintString` (`KismetStringLibrary.Concat_StrStr` (`KismetSystemLibrary.GetDisplayName` self) " 스위치 객체 정보 안넣었어 바보야!!!") true true (struct :`R` 1.0 :`G` 0.051168 :`B` 0.09097 :`A` 1.0) 60.0))))

(event `self.ReceiveTick`
  (params (DeltaSeconds :type "Float (single-precision)"))
  (if (`self.isplay`)
    (if (`self.right`)
      ;[1 1 1] 오른쪽으로 움직이기
      (bind _output_get (set `self.x_location` (+ (`self.x_location`) 2.0)))
      (`SceneComponent.K2_SetRelativeLocation` (`self.StaticMesh`) (`KismetMathLibrary.MakeVector` _output_get) false false)
      (if (>= (`self.x_location`) 200.0)
        (set `self.right` false))
      (else
        ;[1 1 1] 왼쪽으로 움직이기
        (bind _output_get_2 (set `self.x_location` (+ (`self.x_location`) -2.0)))
        (`SceneComponent.K2_SetRelativeLocation` (`self.StaticMesh`) (`KismetMathLibrary.MakeVector` _output_get_2) false false)
        (if (<= (`self.x_location`) 0.0)
          (set `self.right` true))))))

(fn `Do play`
  (params (isplay :type Boolean))
  (returns (bresult :type Boolean))
  (set `self.isplay` isplay)
  (return false))

(fn `EventOverlap`
  (params (IsBegin :type Boolean))
  (set `self.isplay` IsBegin))

(fn `UserConstructionScript`)